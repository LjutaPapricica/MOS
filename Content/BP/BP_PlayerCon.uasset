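; BP_PlayerCon is a player controller that routes input to the player character and sets up the HUD.
; On BeginPlay it caches the controlled pawn as a BP_Player reference, then creates a UI_HUD widget and adds it to the viewport.
; Movement axes are forwarded to movement functions on BP_Player, while the horizontal look axis applies yaw input directly to the controlled pawn.
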(fn ConstructionScript)

(fn CreateWidget
  (bind _returnvalue (UserInterface|CreateWidget "/Game/BP/UI_HUD.UI_HUD_C" self))
  (UserInterface|Viewport|AddtoViewport _returnvalue 0))

(event Input|AxisEvents|InputAxisMoveForward/Backward
  (params (AxisValue :type Float%20%28single-precision%29))
  (Default|MoveForward/Backward (Variables|Default|GetPlayerRefe) AxisValue))

(event Input|AxisEvents|InputAxisMoveRight/Left
  (params (AxisValue :type Float%20%28single-precision%29))
  (Default|MoveRight/Left (Variables|Default|GetPlayerRefe) AxisValue))

(event Input|AxisEvents|InputAxisLookRight/Left
  (params (AxisValue :type Float%20%28single-precision%29))
  (Pawn|Input|AddControllerYawInput (Pawn|GetControlledPawn) AxisValue))

(event EventBeginPlay
  (Utilities|FlowControl|Sequence
    (:then_0
      (Variables|Default|SetPlayerRefe (.AsBP%20Player (Utilities|Casting|CastToBP_Player (Pawn|GetControlledPawn)))))
    (:then_1
      (CallFunction|CreateWidget))))