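; Multiplayer third-person shooter character with a socketed rifle, aim-only hitscan firing, health, score and kill streak, tinted with the game instance's player color.
; Aim, fire and damage go through server-to-multicast events, so the line trace and HP subtraction run inside the multicast.
; Death credits the killer, ragdolls the body, then respawns it at a random named PlayerStart after a delay.
; A separate Trace function measures aim-line range with debug drawing.
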(event Custom|server_AnyDamage
  (params (HP :type Float%20%28single-precision%29) (DamageCauser :type BP%20Player%20Object%20Reference))
  (CallFunction|MulticastAnyDamage HP DamageCauser))

(event Custom|multicast_AnyDamage
  (params (HP :type Float%20%28single-precision%29) (DamageCauser :type BP%20Player%20Object%20Reference))
  (|CollapseGraph_1)
  (if (<= HP 0.0)
    (CallFunction|AddScore DamageCauser)
    (Variables|Default|SetKillStreak 0)
    (Physics|SetSimulatePhysics (Variables|Character|GetMesh) true)
    (Collision|SetCollisionEnabled (Variables|Collision|GetCapsuleComponent) "NoCollision")
    (Utilities|FlowControl|Delay 3.0)
    (|Respawn)))

(fn ConstructionScript
  (Transformation|AttachComponentToComponent (Variables|Default|GetGun) (Variables|Character|GetMesh) "AR4GunSocket" "SnapToTarget" "SnapToTarget" "KeepWorld" true)
  (bind _returnvalue (Rendering|Material|CreateDynamicMaterialInstance (Variables|Character|GetMesh) 0 0 "None" :!class /Script/Engine.PrimitiveComponent))
  (bind _output_get (Variables|Default|SetMI_BodyColor _returnvalue))
  (Rendering|Material|SetVectorParameterValue _output_get "BodyColor" (Variables|/Game/BP/MainGI.MainGI_C|GetPlayerColor (.AsMain%20GI (Utilities|Casting|CastToMainGI (Game|GetGameInstance)))) :!class /Script/Engine.MaterialInstanceDynamic))

(fn MoveForward/Backward
  (params (ScaleValue :type Float%20%28single-precision%29))
  (Pawn|Input|AddMovementInput (Math|Vector|GetForwardVector (Pawn|GetControlRotation :!class /Script/Engine.Pawn)) ScaleValue false))

(fn MoveRight/Left
  (params (ScaleValue :type Float%20%28single-precision%29))
  (Pawn|Input|AddMovementInput (Math|Vector|GetRightVector (Pawn|GetControlRotation :!class /Script/Engine.Pawn)) ScaleValue false))

(fn OnTakeDamage
  (params (Damage :type Float%20%28single-precision%29))
  (bind _output_get (Variables|Default|SetHP (- (Variables|Default|GetHP) Damage)))
  (return _output_get))

(fn AddScore
  (Variables|Default|SetScore (+ (Variables|Default|GetScore) 100))
  (Math|Integer|IncrementInt (Variables|Default|GetKillStreak)))

(fn Trace
  (bind (_start _end) (|CollapseGraph_0_2))
  (bind (_outhit _returnvalue) (Collision|LineTraceByChannel _start _end "TraceTypeQuery1" false 0 "ForOneFrame" true "(R=0.000000,G=1.000000,B=0.103376,A=1.000000)" "(R=0.000000,G=0.000000,B=0.000000,A=0.000000)" 0.0))
  (Variables|Default|SetisTraceHit (Math|Boolean|ORBoolean _returnvalue (.bBlockingHit (Collision|BreakHitResult _outhit)) (.bInitialOverlap (Collision|BreakHitResult _outhit))))
  (Variables|Default|SetTraceRange (Math|Vector|VectorLengthXY (- (.ImpactPoint (Collision|BreakHitResult _outhit)) _start))))

(event Custom|server_fire
  (params (Condition :type Boolean) (Start :type Vector) (End :type Vector))
  ;[1 1 1] Fire
  (CallFunction|MulticastFire Condition Start End))

(event Custom|multicast_fire
  (params (Condition :type Boolean) (Start :type Vector) (End :type Vector))
  ;[1 1 1] Fire
  (if Condition
    (|moromoro)
    (bind (_outhit _returnvalue) (Collision|LineTraceByChannel Start End "TraceTypeQuery1" false 0 "None" true "(R=1.000000,G=0.000000,B=0.000000,A=1.000000)" "(R=0.000000,G=1.000000,B=0.000000,A=1.000000)" 1.0))
    (if _returnvalue
      (bind _hp (CallFunction|OnTakeDamage (.AsBP%20Player (Utilities|Casting|CastToBP_Player (.HitActor (Collision|BreakHitResult _outhit)))) 2e+01))
      (CallFunction|ServerAnyDamage (.AsBP%20Player (Utilities|Casting|CastToBP_Player (.HitActor (Collision|BreakHitResult _outhit)))) _hp self))))

(event Custom|server_Aim
  (params (isAiming :type Boolean) (bUseControllerRotationYaw :type Boolean) (bOrientRotationToMovement :type Boolean) (MaxWalkSpeed :type Float%20%28single-precision%29))
  ;[1 1 1] Aim
  (CallFunction|MulticastAim isAiming bUseControllerRotationYaw bOrientRotationToMovement MaxWalkSpeed))

(event Custom|multicast_Aim
  (params (isAiming :type Boolean) (bUseControllerRotationYaw :type Boolean) (bOrientRotationToMovement :type Boolean) (MaxWalkSpeed :type Float%20%28single-precision%29))
  (bind _charactermovement (Variables|Character|GetCharacterMovement))
  ;[1 1 1] Aim
  (Variables|Default|SetisAiming isAiming)
  (Variables|Default|SetbUseControllerRotationYaw bUseControllerRotationYaw)
  (Variables|/Script/Engine.CharacterMovementComponent|SetbOrientRotationToMovement _charactermovement bOrientRotationToMovement)
  (Variables|/Script/Engine.CharacterMovementComponent|SetMaxWalkSpeed _charactermovement MaxWalkSpeed))

(event Input|ActionEvents|InputActionAim
  (params (Key :type Key%20Structure))
  ;[1 1 1] Aim
  (:Pressed
    (CallFunction|ServerAim true true false 2e+02))
  (:Released
    (CallFunction|ServerAim false false true 7.5e+02)))

(event Input|ActionEvents|InputActionFire
  (params (Key :type Key%20Structure))
  (bind (_start _end) (|CollapseGraph_0))
  ;[1 1 1] Fire
  (:Pressed
    (CallFunction|ServerFire (Variables|Default|GetisAiming) _start _end)))

(event EventBeginPlay
  (Utilities|Time|SetTimerbyEvent (EventDispatchers|CreateEvent :!event Trace) 0.01 true))